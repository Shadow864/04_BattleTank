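; Experimental car actor that is pushed along by physics forces on its four wheel components.
; Every Tick adds the same Force vector to each wheel as a plain, mass-dependent force.
; The graphs contain no input, steering or suspension logic, and BeginPlay and the construction script are empty.
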(event EventBeginPlay)

(event Collision|EventActorBeginOverlap
  (params (OtherActor :type Actor%20Object%20Reference)))

(event EventTick
  (params (DeltaSeconds :type Float%20%28single-precision%29))
  (Physics|AddForce (Variables|Default|GetWheel1) (Variables|Default|GetForce) "None" false)
  (Physics|AddForce (Variables|Default|GetWheel2) (Variables|Default|GetForce) "None" false)
  (Physics|AddForce (Variables|Default|GetWheel3) (Variables|Default|GetForce) "None" false)
  (Physics|AddForce (Variables|Default|GetWheel4) (Variables|Default|GetForce) "None" false))

(fn ConstructionScript)